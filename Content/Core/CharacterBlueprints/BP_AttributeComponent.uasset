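; BP_AttributeComponent is a character attribute component that tracks Health against MaxHealth.
; ApplyHealthChange adds a signed delta, clamps the result between zero and MaxHealth, then broadcasts OnHealthChanged with the new value and requested delta.
; Each branch prints Health on screen in its own color for debugging; reaching zero only adds a death message, with no further death handling.
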(fn `ApplyHealthChange`
  (params (HealthDelta :type "Float (double-precision)" :default -10.0))
  (bind _maxhealth (`self.MaxHealth`))
  (bind _returnvalue (+ (`self.Health`) HealthDelta))
  (if (<= _returnvalue 0.0)
    (`KismetSystemLibrary.PrintString` "YOU DIED!!!")
    (bind _output_get (set `self.Health` 0.0))
    (`KismetSystemLibrary.PrintString` (`KismetStringLibrary.Conv_DoubleToString` _output_get) true true (struct :`R` 1.0 :`G` 1.0 :`B` 1.0 :`A` 1.0))
    (`self.OnHealthChanged` null self _output_get HealthDelta)
    (elif (>= _returnvalue _maxhealth)
      (bind _output_get_2 (set `self.Health` _maxhealth))
      (`KismetSystemLibrary.PrintString` (`KismetStringLibrary.Conv_DoubleToString` _output_get_2) true true (struct :`G` 1.0 :`B` 0.119571 :`A` 1.0))
      (`self.OnHealthChanged` null self _output_get_2 HealthDelta)
      (else
        (bind _output_get_3 (set `self.Health` _returnvalue))
        (`KismetSystemLibrary.PrintString` (`KismetStringLibrary.Conv_DoubleToString` _output_get_3) true true (struct :`R` 1.0 :`B` 0.112927 :`A` 1.0))
        (`self.OnHealthChanged` null self _output_get_3 HealthDelta)))))