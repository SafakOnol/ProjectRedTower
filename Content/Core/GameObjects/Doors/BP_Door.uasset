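; BP_Door is a door actor that opens when something begins overlapping its Box component, either swinging or sliding according to the IsSlidingDoor flag.
; The overlap calls OnDoorOpen, which plays the DoorOpening timeline and passes its position as alpha to the hinge and slide functions.
; Each function checks the flag, then lerps the Scene component's relative yaw or its location along a normalized direction.
; The graph has no closing logic.
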(event `OnDoorOpen`
  (bind (_direction _position) (`Timeline|DoorOpening`)
    (:`Update`
      (`self.SetHingePosition` _position)
      (`self.SetSlidePosition` _position))))

(event `self.Box.OnComponentBeginOverlap`
  (params (OverlappedComponent :type "PrimitiveComponent Object Reference") (OtherActor :type "Actor Object Reference") (OtherComp :type "PrimitiveComponent Object Reference") (OtherBodyIndex :type Integer) (bFromSweep :type Boolean) (SweepResult :type "HitResult Structure (by ref)"))
  (`self.OnDoorOpen`))

(fn `SetHingePosition`
  (params (Alpha :type "Float (double-precision)") (MaxHingeRotation :type "Float (double-precision)" :default -90.0))
  (if (not (`self.bIsSlidingDoor`))
    (`SceneComponent.K2_SetRelativeRotation` (`self.Scene`) (`KismetMathLibrary.MakeRotator` 0.0 0.0 (`KismetMathLibrary.Lerp` 0.0 MaxHingeRotation Alpha)) false false)))

(fn `SetSlidePosition`
  (params (Alpha :type "Float (double-precision)") (MaxSlideDistance :type "Float (double-precision)" :default 125.0) (Direction :type "Vector Structure" :default (0.0 1.0 0.0)))
  (if (`self.bIsSlidingDoor`)
    (`SceneComponent.K2_SetRelativeLocation` (`self.Scene`) (* (`KismetMathLibrary.Lerp` 0.0 MaxSlideDistance Alpha) (`KismetMathLibrary.Normal` Direction)) false false)))

(fn `UserConstructionScript`)