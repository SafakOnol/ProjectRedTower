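; BP_ProjectileCannon is a cannon actor that periodically fires BP_Projectile.
; After a startup delay on BeginPlay, a looping timer spawns a projectile at the actor's location and rotation.
; Tick turns the Arrow component toward the first player pawn every frame, while the spawn transform reads the actor's rotation rather than the Arrow's.
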(event `self.ReceiveBeginPlay`
  (`KismetSystemLibrary.Delay` 5.0)
  (`KismetSystemLibrary.K2_SetTimerDelegate` (delegate `OnTImerElapsed`) 2.0 true))

(event `OnTImerElapsed`
  (`|SpawnActorFromClass` "/Game/Core/Projectile/BP_Projectile.BP_Projectile_C" (`KismetMathLibrary.MakeTransform` (`self.K2_GetActorLocation`) (`self.K2_GetActorRotation`)) "Undefined" "MultiplyWithRoot" null null))

(event `self.ReceiveTick`
  (params (DeltaSeconds :type "Float (single-precision)"))
  (`SceneComponent.K2_SetWorldRotation` (`self.Arrow`) (`KismetMathLibrary.FindLookAtRotation` (`self.K2_GetActorLocation`) (`self.K2_GetActorLocation` (`GameplayStatics.GetPlayerPawn` 0))) false false))

(fn `UserConstructionScript`)